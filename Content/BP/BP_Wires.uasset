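; BP_Wires is a wire-connection puzzle that manages four BP_Wire child actors and detects when all are attached successfully.
; The construction script gathers the wires, colors each by index from a Colors array, and shuffles their attach locations among them.
; At BeginPlay it binds to each wire's OnAttached event, which checks every wire's IsSuccess flag and prints a completion message when all are true.
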(event Custom|OnAttached_Event
  (if (CallFunction|IsCompleted)
    (Development|PrintString "Completed!")))

(event EventBeginPlay
  (for _array_element (Variables|Default|Getwires)
    (EventDispatchers|AssignOnAttached _array_element (delegate Custom|OnAttached_Event))))

(event Collision|EventActorBeginOverlap
  (params (OtherActor :type Actor%20Object%20Reference)))

(event EventTick
  (params (DeltaSeconds :type Float%20%28single-precision%29)))

(fn ConstructionScript
  (Utilities|FlowControl|Sequence
    (:then_0
      (for _array_element (Utilities|Array|MakeArray (Variables|Default|GetChildActor1) (Variables|Default|GetChildActor2) (Variables|Default|GetChildActor3) (Variables|Default|GetChildActor))
        (bind _asbp_wire (Utilities|Casting|CastToBP_Wire (Variables|/Script/Engine.ChildActorComponent|GetChildActor _array_element)))
        (Utilities|Array|Add (Variables|Default|Getwires) _asbp_wire)))
    (:then_1
      (for (_array_element_2 _array_index) (Variables|Default|Getwires)
        (Default|SetWireColor _array_element_2 (Utilities|Array|Get(acopy) (Variables|Default|Getcolors) _array_index))))
    (:then_2
      (CallFunction|ShuffleEndLocations))))

(fn ShuffleEndLocations
  (Utilities|FlowControl|Sequence
    (:then_0
      (for _array_element (Variables|Default|Getwires)
        (Utilities|Array|Add (LocalVariables|Getlocation_l) (Default|GetAttachLocation _array_element))))
    (:then_1
      (Utilities|Array|Shuffle (LocalVariables|Getlocation_l)))
    (:then_2
      (for (_array_element_2 _array_index) (Variables|Default|Getwires)
        (Default|SetAttachLocation _array_element_2 (Utilities|Array|Get(acopy) (LocalVariables|Getlocation_l) _array_index))))))

(fn IsCompleted
  (for _array_element (Variables|Default|Getwires)
    (Utilities|Array|Add (LocalVariables|GetisSuccess_l) (Variables|/Game/BP/BP_Wire.BP_Wire_C|GetisSuccess _array_element)))
  (return (not (Utilities|Array|ContainsItem (LocalVariables|GetisSuccess_l) false))))