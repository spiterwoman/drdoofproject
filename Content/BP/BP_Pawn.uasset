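; Player pawn for a wire-connecting minigame that views the BP_Wires actor and shows the mouse cursor.
; Pressing left mouse traces under the cursor to grab a BP_Wire; releasing traces again to attach it to a valid wire, or resets it.
; While held, Tick moves the wire's end to where the cursor ray intersects a plane through the wire, facing along its forward vector.
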(event Custom|StartGrab
  (bind _returnvalue (Game|GetPlayerState 0))
  (bind _returnvalue_2 (Game|GetPlayerController _returnvalue))
  (bind (_worldlocation _worlddirection) (Game|Player|ConvertMouseLocationToWorldSpace _returnvalue_2))
  (bind (_outhit _returnvalue_3) (Collision|LineTraceByChannel _worldlocation (+ _worldlocation (* _worlddirection 1e+03)) "TraceTypeQuery1" false 0 "ForOneFrame"))
  (if _returnvalue_3
    (bind _asbp_wire (Utilities|Casting|CastToBP_Wire (.HitActor (Collision|BreakHitResult _outhit))))
    (if (Default|CanGrab _asbp_wire (.HitComponent (Collision|BreakHitResult _outhit)))
      (bind _output_get (Variables|Default|SetgrabWire _asbp_wire))
      (Default|StartGrab _output_get))))

(event Custom|EndGrab
  (bind _returnvalue (Game|GetPlayerState 0))
  (bind _returnvalue_2 (Game|GetPlayerController _returnvalue))
  (bind (_worldlocation _worlddirection) (Game|Player|ConvertMouseLocationToWorldSpace _returnvalue_2))
  (Variables|Default|GetgrabWire
    (:then
      (bind (_outhit _returnvalue_3) (Collision|LineTraceByChannel _worldlocation (+ _worldlocation (* _worlddirection 1e+03)) "TraceTypeQuery1" false 0 "ForOneFrame"))
      (if _returnvalue_3
        (bind _asbp_wire (Utilities|Casting|CastToBP_Wire (.HitActor (Collision|BreakHitResult _outhit)))
          (:then
            (if (Default|CanAttach _asbp_wire (.HitComponent (Collision|BreakHitResult _outhit)))
              (Default|Attach (Variables|Default|GetgrabWire) _asbp_wire)
              (Variables|Default|SetgrabWire 0)
              (else
                (CallFunction|ResetGrab))))
          (:CastFailed
            (CallFunction|ResetGrab)))
        (else
          (CallFunction|ResetGrab))))
    (:else)))

(event Custom|UpdateGrab
  (bind _returnvalue (Game|GetPlayerState 0))
  (bind _returnvalue_2 (Game|GetPlayerController _returnvalue))
  (bind (_worldlocation _worlddirection) (Game|Player|ConvertMouseLocationToWorldSpace _returnvalue_2))
  (bind _grabwire (Variables|Default|GetgrabWire)
    (:then
      (if (.ReturnValue (Class|KismetMathLibrary|LinePlaneIntersectionOriginNormal _worldlocation (+ _worldlocation (* _worlddirection 1e+03)) (Transformation|GetActorLocation _grabwire) (Transformation|GetActorForwardVector _grabwire)))
        (Default|SetEndLocation _grabwire (.Intersection (Class|KismetMathLibrary|LinePlaneIntersectionOriginNormal _worldlocation (+ _worldlocation (* _worlddirection 1e+03)) (Transformation|GetActorLocation _grabwire) (Transformation|GetActorForwardVector _grabwire))))))
    (:else)))

(event Custom|ResetGrab
  (bind _grabwire (Variables|Default|GetgrabWire)
    (:then
      (Default|Reset _grabwire)
      (Variables|Default|SetgrabWire 0))
    (:else)))

(event EventBeginPlay
  (bind _returnvalue (Game|GetPlayerState 0))
  (bind _returnvalue_2 (Game|GetPlayerController _returnvalue))
  (bind _outactors (Actor|GetAllActorsOfClass "/Game/BP/BP_Wires.BP_Wires_C"))
  (Game|Player|SetViewTargetwithBlend _returnvalue_2 (Utilities|Array|Get(acopy) _outactors) 0.0 "VTBlend_Linear" 0.0 false)
  (Variables|/Script/Engine.PlayerController|SetbShowMouseCursor _returnvalue_2 true))

(event Collision|EventActorBeginOverlap
  (params (OtherActor :type Actor%20Object%20Reference)))

(event EventTick
  (params (DeltaSeconds :type Float%20%28single-precision%29))
  (CallFunction|UpdateGrab))

(event Input|MouseEvents|LeftMouseButton
  (params (Key :type Key%20Structure :default "None"))
  (:Pressed
    (CallFunction|StartGrab))
  (:Released
    (CallFunction|EndGrab)))

(fn ConstructionScript)